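; BP_Boss is the boss enemy Blueprint, whose death triggers the game's win sequence.
; When its HealthComponent fires OnDeath, a sequence creates the BP_GameWin widget, shows the mouse cursor and switches input to UI only.
; It then stops and releases the boss music held on BP_GrimGameMode and plays a one-shot 2D boss death event.
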(event `self.ReceiveBeginPlay`)

(event `self.HealthComponent.OnDeath`
  (bind _returnvalue (`GameplayStatics.GetPlayerController` 0))
  (`|ExecutionSequence`
    (:`then_0`
      (bind _returnvalue_2 (`|CreateWidget` "/Game/Blueprints/UI/BP_GameWin.BP_GameWin_C" _returnvalue))
      (`UserWidget.AddToViewport` _returnvalue_2 0)
      (set `PlayerController.bShowMouseCursor` true _returnvalue)
      (`WidgetBlueprintLibrary.SetInputMode_UIOnlyEx` _returnvalue null))
    (:`then_1`
      ;[1 1 1] Stop boss music
      (bind _asbp_grim_game_mode (cast `/Game/Blueprints/GameEssentials/BP_GrimGameMode` (`GameplayStatics.GetGameMode`)))
      (`FMODBlueprintStatics.EventInstanceStop` (`/Game/Blueprints/GameEssentials/BP_GrimGameMode.BossMusic` _asbp_grim_game_mode) true))
    (:`then_2`
      (bind _returnvalue_3 (`FMODBlueprintStatics.PlayEvent2D` "/Game/FMOD/Events/Enemies/BossDies.BossDies"))
      (`FMODBlueprintStatics.EventInstancePlay` _returnvalue_3)
      (`FMODBlueprintStatics.EventInstanceRelease` _returnvalue_3))))

(fn `UserConstructionScript`
  (`parent.UserConstructionScript`))