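; Base enemy character that scales with game difficulty, reacts to hits and handles its death.
; On BeginPlay it maps the game mode's difficulty to a random strength, which sets capsule scale, damage and max health for non-bosses.
; HealthComponent events drive damage numbers, blood effects and death, with a chance to drop a ground-traced soul pickup.
; Death unpossesses the AI, then plays any death montage before destroying the actor.
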(event `self.ReceiveBeginPlay`
  (bind _asbp_grim_game_mode (cast `/Game/Blueprints/GameEssentials/BP_GrimGameMode` (`GameplayStatics.GetGameMode`)))
  (set `self.As BP Grim Game Mode` _asbp_grim_game_mode)
  (`self.MapDifficulty`)
  (if (not (`self.isBoss`))
    (`self.SetEnemyStrength`)))

(event `SetEnemyStrength`
  (bind _randomstrength (`self.RandomStrength`))
  (bind _healthcomponent (`self.HealthComponent`))
  (`SceneComponent.SetWorldScale3D` (`self.CapsuleComponent`) (`KismetMathLibrary.Conv_DoubleToVector` (`KismetMathLibrary.FClamp` (* (`self.RandomStrength`) 0.8) 0.8 1.5)))
  (set `self.BaseDamage` _randomstrength)
  (bind _output_get (set `HealthComponent.MaxHealth` (* (`HealthComponent.MaxHealth` _healthcomponent) (* _randomstrength 2.0)) _healthcomponent))
  (set `HealthComponent.CurrentHealth` _output_get (`self.HealthComponent`)))

(event `MapDifficulty`
  (bind _returnvalue (`KismetMathLibrary.MapRangeClamped` (`KismetMathLibrary.Conv_IntToDouble` (`GrimGameMode.CurrentDifficulty` (`self.As BP Grim Game Mode`))) 0.0 100.0 0.8 2.0))
  (set `self.RandomStrength` (`KismetMathLibrary.RandomFloatInRange` _returnvalue (+ _returnvalue 0.2))))

(event `self.HealthComponent.OnHit`
  (params (DamageAmount :type "Float (single-precision)") (CritDamage :type Boolean))
  (bind _returnvalue (`self.GetComponentByClass` "/Game/Materials/Blood/AC_Blood_Effect.AC_Blood_Effect_C"))
  (bind _returnvalue_2 (`KismetMathLibrary.FTrunc` DamageAmount))
  (bind _returnvalue_3 (`self.K2_GetActorLocation`))
  (bind _returnvalue_4 (`KismetMathLibrary.Conv_VectorToTransform` _returnvalue_3))
  (if (not (`self.isDead`))
    (`|ExecutionSequence`
      (:`then_0`
        (if CritDamage
          (`|SpawnActorFromClass` "/Game/UI/DamageNumbers/BP_CritDamageNumberActor.BP_CritDamageNumberActor_C" _returnvalue_4 "Undefined" "OverrideRootScale" null _returnvalue_2 null)
          (else
            (`|SpawnActorFromClass` "/Game/UI/DamageNumbers/BP_DamageNumberActor.BP_DamageNumberActor_C" _returnvalue_4 "Undefined" "OverrideRootScale" null _returnvalue_2 null))))
      (:`then_1`
        (`/Engine/EditorBlueprintResources/StandardMacros.IsValid` _returnvalue
          (:`Is Valid`
            (`/Game/Materials/Blood/AC_Blood_Effect.Blood Effect` _returnvalue _returnvalue_3 (0.0 0.0 0.0))))))))

(event `/Game/Blueprints/Interfaces/BI_ExplosiveDamage.ExplosiveDamage`
  (`HealthComponent.TakeDamage` (`self.HealthComponent`) 20.0 false))

(event `self.HealthComponent.OnDeath`
  (bind _returnvalue (`self.K2_GetActorLocation`))
  ;[1 1 1] Drop loot function
  (if (not (`self.isDead`))
    (set `self.isDead` true)
    (`|ExecutionSequence`
      (:`then_0`
        (if (<= (`KismetMathLibrary.RandomFloatInRange` 0.0 100.0) 10.0)
          (bind _outhit (`KismetSystemLibrary.LineTraceSingle` _returnvalue (- _returnvalue (0.0 0.0 200.0)) "TraceTypeQuery1" false (`|MakeArray` (`GameplayStatics.GetPlayerCharacter` 0) :!type "Actor Object Reference")))
          (`|SpawnActorFromClass` "/Game/Blueprints/Items/BP_SoulPickup.BP_SoulPickup_C" (`KismetMathLibrary.MakeTransform` (`.Location` (`GameplayStatics.BreakHitResult` _outhit)) (`KismetMathLibrary.MakeRotator` 0.0 0.0 (`KismetMathLibrary.RandomFloatInRange` 0.0 360.0))) "AdjustIfPossibleButDontSpawnIfColliding" "OverrideRootScale" null null)))
      (:`then_1`
        (`self.DeathEvent`)))))

(event `DeathEvent`
  (bind _returnvalue (`AIBlueprintHelperLibrary.GetAIController` self))
  (bind _deathmontage (`HealthComponent.DeathMontage` (`self.HealthComponent`)))
  ;[1 1 1] Drop loot function
  (`/Engine/EditorBlueprintResources/StandardMacros.IsValid` _returnvalue
    (:`Is Valid`
      (`Controller.UnPossess` _returnvalue)
      (`/Engine/EditorBlueprintResources/StandardMacros.IsValid` _deathmontage
        (:`Is Valid`
          (`self.PlayAnimMontage` _deathmontage)
          (`PrimitiveComponent.SetCollisionResponseToChannel` (`self.CapsuleComponent`) "ECC_Pawn" "ECR_Ignore")
          (`KismetSystemLibrary.Delay` 2.5)
          (`self.K2_DestroyActor`))))))

(event `SetMovementSpeed`
  (params (NewMovementSpeed :type "Float (double-precision)"))
  (set `CharacterMovementComponent.MaxWalkSpeed` NewMovementSpeed (`self.CharacterMovement`)))

(fn `UserConstructionScript`)