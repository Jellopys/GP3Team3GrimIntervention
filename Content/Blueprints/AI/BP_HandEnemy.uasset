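; BP_HandEnemy is an AI hand enemy with a ground slam area attack against the player.
; GroundSlam turns on the SlamSphere's overlap, fires the slam VFX and uses a timeline to grow the sphere's radius like a shockwave.
; Overlapping the cached player applies SlamDamage through its HealthComponent, with a HitActors list limiting it to one hit per slam.
; When the timeline finishes, collision is disabled and the hit list clears.
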(event `self.ReceiveBeginPlay`
  (`parent.ReceiveBeginPlay`)
  (bind _asbp_player_character (cast `/Game/Blueprints/Player/BP_PlayerCharacter` (`GameplayStatics.GetPlayerPawn` 0)))
  (set `self.As BP Player Character` _asbp_player_character))

(event `GroundSlam`
  (bind _slamsphere (`self.SlamSphere`))
  (`PrimitiveComponent.SetCollisionResponseToAllChannels` (`self.SlamSphere`) "ECR_Overlap")
  (`ActorComponent.Activate` (`self.SlamVFX`) true)
  (bind (_direction _newtrack_0) (`Timeline|Timeline` :!via `PlayFromStart`)
    (:`Update`
      (`SphereComponent.SetSphereRadius` _slamsphere (`KismetMathLibrary.Lerp` (`self.StartRadius`) (`self.EndRadius`) _newtrack_0) true))
    (:`Finished`
      (`PrimitiveComponent.SetCollisionResponseToAllChannels` _slamsphere "ECR_Ignore")
      (`KismetArrayLibrary.Array_Clear` (`self.HitActors`)))))

(event `self.SlamSphere.OnComponentBeginOverlap`
  (params (OverlappedComponent :type "PrimitiveComponent Object Reference") (OtherActor :type "Actor Object Reference") (OtherComp :type "PrimitiveComponent Object Reference") (OtherBodyIndex :type Integer) (bFromSweep :type Boolean) (SweepResult :type "HitResult Structure (by ref)"))
  (bind _returnvalue (`self.GetComponentByClass` OtherActor "/Script/GP3Team3.HealthComponent"))
  (if (== OtherActor (`self.As BP Player Character`))
    (if (not (`KismetArrayLibrary.Array_Contains` (`self.HitActors`) OtherActor))
      (`/Engine/EditorBlueprintResources/StandardMacros.IsValid` _returnvalue
        (:`Is Valid`
          (`HealthComponent.TakeDamage` _returnvalue (`self.SlamDamage`) false)
          (`KismetArrayLibrary.Array_Add` (`self.HitActors`) OtherActor))))))

(fn `UserConstructionScript`
  (`parent.UserConstructionScript`))