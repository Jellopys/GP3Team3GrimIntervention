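; Boss enemy Blueprint that shows a boss health bar on BeginPlay and takes fixed damage from explosive hits through its HealthComponent.
; Toggled scythe collision damages the player on overlap, tracking hit actors so each is hurt once until collision is disabled.
; On death it shows the win widget with UI-only input, clears the game mode's boss music reference before setting its death parameter, and plays a death audio event.
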(event `/Game/Blueprints/Interfaces/BI_ExplosiveDamage.ExplosiveDamage`
  (`HealthComponent.TakeDamage` (`self.HealthComponent`) 20.0 false))

(event `self.ReceiveBeginPlay`
  (`parent.ReceiveBeginPlay`)
  (bind _asbp_player_character (cast `/Game/Blueprints/Player/BP_PlayerCharacter` (`GameplayStatics.GetPlayerPawn` 0)))
  (set `self.As BP Player Character` _asbp_player_character)
  (bind _returnvalue (`|GenericCreateObject` "/Game/Blueprints/UI/WB_BossHealthBar.WB_BossHealthBar_C"))
  (set `/Game/Blueprints/UI/WB_BossHealthBar.Boss` self _returnvalue)
  (`UserWidget.AddToViewport` _returnvalue 0))

(event `self.HealthComponent.OnDeath`
  (bind _returnvalue (`GameplayStatics.GetPlayerController` 0))
  (`|ExecutionSequence`
    (:`then_0`
      (bind _returnvalue_2 (`|CreateWidget` "/Game/Blueprints/UI/BP_GameWin.BP_GameWin_C" _returnvalue))
      (`UserWidget.AddToViewport` _returnvalue_2 0)
      (set `PlayerController.bShowMouseCursor` true _returnvalue)
      (`WidgetBlueprintLibrary.SetInputMode_UIOnlyEx` _returnvalue null))
    (:`then_1`
      ;[1 1 1] Stop boss music
      (bind _asbp_grim_game_mode (cast `/Game/Blueprints/GameEssentials/BP_GrimGameMode` (`GameplayStatics.GetGameMode`)))
      (bind _output_get (set `/Game/Blueprints/GameEssentials/BP_GrimGameMode.BossMusic` (struct) _asbp_grim_game_mode))
      (`FMODBlueprintStatics.EventInstanceSetParameter` _output_get "BossDies" (`self.TriggerBossDead`)))
    (:`then_2`
      (bind _returnvalue_3 (`FMODBlueprintStatics.PlayEvent2D` "/Game/FMOD/Events/Enemies/BossDies.BossDies"))
      (`FMODBlueprintStatics.EventInstancePlay` _returnvalue_3)
      (`FMODBlueprintStatics.EventInstanceRelease` _returnvalue_3))))

(event `EnableScytheCollision`
  (`PrimitiveComponent.SetCollisionResponseToAllChannels` (`self.SM_scythe_blockout`) "ECR_Overlap"))

(event `DisableScytheCollision`
  (`PrimitiveComponent.SetCollisionResponseToAllChannels` (`self.SM_scythe_blockout`) "ECR_Ignore")
  (`KismetArrayLibrary.Array_Clear` (`self.Other Actor`)))

(event `self.SM_scythe_blockout.OnComponentBeginOverlap`
  (params (OverlappedComponent :type "PrimitiveComponent Object Reference") (OtherActor :type "Actor Object Reference") (OtherComp :type "PrimitiveComponent Object Reference") (OtherBodyIndex :type Integer) (bFromSweep :type Boolean) (SweepResult :type "HitResult Structure (by ref)"))
  (bind _returnvalue (`self.GetComponentByClass` OtherActor "/Script/GP3Team3.HealthComponent"))
  (if (== OtherActor (`self.As BP Player Character`))
    (if (not (`KismetArrayLibrary.Array_Contains` (`self.Other Actor`) OtherActor))
      (`/Engine/EditorBlueprintResources/StandardMacros.IsValid` _returnvalue
        (:`Is Valid`
          (`HealthComponent.TakeDamage` _returnvalue (`self.ScytheAOEDMG`) false)
          (`KismetArrayLibrary.Array_Add` (`self.Other Actor`) OtherActor))))))

(fn `UserConstructionScript`
  (`parent.UserConstructionScript`))