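; Player character for a scythe-wielding action game with combo attacks, dash, kick, aura, pause and death screens.
; Montage notifies toggle weapon overlap, which deals crit-capable damage from GameInstance stats and GameMode temporary bonuses.
; Powerup flags modify damage and currency loss, while hits and actions trigger FMOD audio and UI.
; Tick also handles stamina speed penalties and dither-fades meshes between camera and player via sphere traces and dynamic materials.
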(event `/Game/Blueprints/Interfaces/BI_ExplosiveDamage.ExplosiveDamage`
  (`HealthComponent.TakeDamage` (`self.HealthComponent`) 5.0 false))

(event `self.ReceiveBeginPlay`
  ;[1 0.008564 0 1 50] BEGIN PLAY
  (`|ExecutionSequence`
    (:`then_0`
      (bind _returnvalue (`|CreateWidget` "/Game/Blueprints/UI/WB_PlayerHUD.WB_PlayerHUD_C"))
      (bind _output_get (set `self.PlayerHudRef` _returnvalue))
      (`UserWidget.AddToViewport` _output_get 0))
    (:`then_1`
      (bind _returnvalue_2 (`AddComponent|NODE_AddPostProcessComponent-0`))
      (bind _output_get_2 (set `self.CameraPostProcess` _returnvalue_2))
      (setmembers `PostProcessSettings` :`StructRef` (`PostProcessComponent.Settings` _output_get_2) :`DepthOfFieldFstop` (`self.Aperture (F-stop)`) :`DepthOfFieldSensorWidth` (`self.Sensor Width (Mm)`) :`DepthOfFieldFocalDistance` (`SpringArmComponent.TargetArmLength` (`self.SpringArm`))))
    (:`then_2`
      (bind _asbp_grim_game_instance (cast `/Game/Blueprints/GameEssentials/BP_GrimGameInstance` (`GameplayStatics.GetGameInstance`)))
      (set `self.As BP Grim Game Instance` _asbp_grim_game_instance))
    (:`then_3`
      (bind _asgrim_game_mode (cast `GrimGameMode` (`GameplayStatics.GetGameMode`)))
      (set `self.As Grim Game Mode` _asgrim_game_mode))))

(event `self.ReceiveTick`
  (params (DeltaSeconds :type "Float (single-precision)"))
  (bind _returnvalue (`self.K2_GetActorLocation`))
  (bind _meshtoditherfloat (`self.MeshToDitherFLoat`))
  (bind _meshtoditherfloat_2 (`self.MeshToDitherFLoat`))
  (bind _as_grim_game_mode (`self.As Grim Game Mode`))
  (bind _as_bp_grim_game_instance (`self.As BP Grim Game Instance`))
  (bind _thisframehits (`self.ThisFrameHits`))
  (bind _returnvalue_2 (`SceneComponent.K2_GetComponentLocation` (`self.Camera`)))
  ;[1 0.5012 0.7398 1 50] TICK
  (`|ExecutionSequence`
    (:`then_0`
      ;[1 0.433 0.3832 1 50] DASH
      ;;[1 1 1] DashFX Condition
      (if (`self.hasDashDamage`)
        (`FXSystemComponent.SetFloatParameter` (`self.FX_Dash`) "User.hasDamage" 0.2)))
    (:`then_1`
      ;[0.6348 1 0.9801 1 35] Fire sequence every 5 seconds
      (bind _output_get (set `self.timerCounter` (+ DeltaSeconds (`self.timerCounter`))))
      (if (>= _output_get 5.0)
        (set `self.timerCounter` 0.0)
        (`|ExecutionSequence`
          (:`then_0`
            ;[0 1 0.3836 1 20] Add 1 temp damage if player has Patient Combat (every 5 sec)
            (if (`self.hasPatientCombat`)
              (set `GrimGameMode.TileTempDamage` (+ (`GrimGameMode.TileTempDamage` _as_grim_game_mode) 1.0) _as_grim_game_mode))))))
    (:`then_2`
      ;[1 1 1] Fade Objs
      (bind _outhits (`KismetSystemLibrary.SphereTraceMulti` _returnvalue_2 _returnvalue 115.0 "TraceTypeQuery1"))
      (for _array_element _outhits
        (if (< (`KismetMathLibrary.DegAcos` (`KismetMathLibrary.Dot_VectorVector` (`KismetMathLibrary.Normal` (- (`.ImpactPoint` (`GameplayStatics.BreakHitResult` _array_element)) _returnvalue)) (`KismetMathLibrary.Normal` (- _returnvalue_2 _returnvalue)))) 30.0)
          (bind _asstatic_mesh_component (cast `StaticMeshComponent` (`.HitComponent` (`GameplayStatics.BreakHitResult` _array_element))))
          (bind _returnvalue_3 (`PrimitiveComponent.GetMaterial` _asstatic_mesh_component 0))
          (bind _returnvalue_4 (`KismetSystemLibrary.GetDisplayName` _returnvalue_3))
          (bind _returnvalue_5 (`PrimitiveComponent.CreateDynamicMaterialInstance` _asstatic_mesh_component 0 _returnvalue_3 (`KismetStringLibrary.Conv_StringToName` _returnvalue_4)))
          (if (`KismetStringLibrary.Contains` _returnvalue_4 "Fade")
            (`MaterialInstanceDynamic.K2_GetScalarParameterValueByInfo` _returnvalue_5 (`MaterialInterface.GetParameterInfo` _returnvalue_5 "GlobalParameter" "Dither Fade Amount" null))
            (`KismetArrayLibrary.Array_AddUnique` (`self.PreviousHits`) _asstatic_mesh_component)
            (`KismetArrayLibrary.Array_AddUnique` (`self.ThisFrameHits`) _asstatic_mesh_component)
            (if (not (`BlueprintMapLibrary.Map_Contains` _meshtoditherfloat _asstatic_mesh_component))
              (`BlueprintMapLibrary.Map_Add` _meshtoditherfloat _asstatic_mesh_component -1.0)))))
      (for _array_element_2 (`self.PreviousHits`)
        (`/Engine/EditorBlueprintResources/StandardMacros.IsValid` _array_element_2
          (:`Is Valid`
            (if (`KismetArrayLibrary.Array_Contains` _thisframehits _array_element_2)
              (bind _value (`BlueprintMapLibrary.Map_Find` _meshtoditherfloat_2 _array_element_2))
              (bind _returnvalue_6 (`KismetMathLibrary.FClamp` (+ _value (* (`self.FadeOut Multiplier`) DeltaSeconds)) -1.0 0.15))
              (`BlueprintMapLibrary.Map_Add` _meshtoditherfloat_2 _array_element_2 _returnvalue_6)
              (bind _returnvalue_7 (`PrimitiveComponent.GetMaterial` _array_element_2 0))
              (`/Engine/EditorBlueprintResources/StandardMacros.IsValid` _returnvalue_7
                (:`Is Valid`
                  (bind _returnvalue_8 (`PrimitiveComponent.CreateDynamicMaterialInstance` _array_element_2 0 _returnvalue_7 (`KismetStringLibrary.Conv_StringToName` (`KismetSystemLibrary.GetDisplayName` _returnvalue_7))))
                  (`MaterialInstanceDynamic.SetScalarParameterValueByInfo` _returnvalue_8 (make `MaterialParameterInfo` "Dither Fade Amount") _returnvalue_6)))
              (else
                (bind _returnvalue_9 (`KismetMathLibrary.FClamp` (- _value (* (`self.FadeIn Multiplier`) DeltaSeconds)) -1.0 0.15))
                (`BlueprintMapLibrary.Map_Add` _meshtoditherfloat_2 _array_element_2 _returnvalue_9)
                (bind _returnvalue_10 (`PrimitiveComponent.GetMaterial` _array_element_2 0))
                (`/Engine/EditorBlueprintResources/StandardMacros.IsValid` _returnvalue_10
                  (:`Is Valid`
                    (bind _returnvalue_11 (`PrimitiveComponent.CreateDynamicMaterialInstance` _array_element_2 0 _returnvalue_10 (`KismetStringLibrary.Conv_StringToName` (`KismetSystemLibrary.GetDisplayName` _returnvalue_10))))
                    (`MaterialInstanceDynamic.SetScalarParameterValueByInfo` _returnvalue_11 (make `MaterialParameterInfo` "Dither Fade Amount") _returnvalue_9)
                    (if (<= _returnvalue_9 -1.0)
                      (`BlueprintMapLibrary.Map_Remove` (`self.MeshToDitherFLoat`) _array_element_2)
                      (`KismetArrayLibrary.Array_RemoveItem` (`self.PreviousHits`) _array_element_2)))))))))
      (`KismetArrayLibrary.Array_Clear` _thisframehits))
    (:`then_3`
      (if (<= (`self.CurrentStamina`) 100.0)
        (if (not (`self.StaminaDepleted`))
          (set `self.StaminaDepleted` true)
          (`GrimGameInstance.UpgradeStat` _as_bp_grim_game_instance -250.0 "MovementSpeed")
          (set `self.StaminaFull` false))))
    (:`then_4`
      (if (>= (`self.CurrentStamina`) 10.0)
        (if (not (`self.StaminaFull`))
          (set `self.StaminaFull` true)
          (`GrimGameInstance.UpgradeStat` _as_bp_grim_game_instance 250.0 "MovementSpeed")
          (set `self.StaminaDepleted` false))))))

(event `Key|P`
  (params (Key :type "Key Structure"))
  ;[0.5222 0.3457 1 1 50] POWERUP CHEAT (HOOKED)
  (:`Pressed`
    (`|SpawnActorFromClass` "/Game/Blueprints/PowerUps/BP_PowerUpChest.BP_PowerUpChest_C" (`KismetMathLibrary.Conv_VectorToTransform` (`self.K2_GetActorLocation`)) "Undefined" "OverrideRootScale" null null)))

(event `self.OnPlayerDeath`
  (bind _returnvalue (`GameplayStatics.GetPlayerController` 0))
  ;[1 1 1] Player death
  (bind _returnvalue_2 (`|CreateWidget` "/Game/Blueprints/UI/BP_GameOver.BP_GameOver_C"))
  (`UserWidget.AddToViewport` _returnvalue_2 0)
  (set `PlayerController.bShowMouseCursor` true _returnvalue)
  (`WidgetBlueprintLibrary.SetInputMode_UIOnlyEx` _returnvalue null)
  (`UserWidget.PlayAnimation` _returnvalue_2 (`/Game/Blueprints/UI/BP_GameOver.FadeIn` _returnvalue_2) 0.0 1 "Forward" 1.0 false)
  ;;[1 1 1] Play Death Sound
  (bind _returnvalue_3 (`FMODBlueprintStatics.PlayEvent2D` "/Game/FMOD/Events/Player/Die.Die"))
  (`FMODBlueprintStatics.EventInstancePlay` _returnvalue_3)
  (`FMODBlueprintStatics.EventInstanceRelease` _returnvalue_3)
  ;[1 1 1] Turn off Low Health effect
  (bind _asbp_grim_game_mode (cast `/Game/Blueprints/GameEssentials/BP_GrimGameMode` (`GameplayStatics.GetGameMode`)))
  (`/Game/Blueprints/GameEssentials/BP_GrimGameMode.TurnOffLowHealth` _asbp_grim_game_mode false))

(event `self.OnDash`
  (params (Pos :type "Vector Structure") (Rot :type "Rotator Structure"))
  ;[1 0.433 0.3832 1 50] DASH
  ;;[1 1 1] DashFX
  (`ActorComponent.SetActive` (`self.FX_Dash`) true false)
  (`PrimitiveComponent.SetCollisionResponseToAllChannels` (`self.SkeletalMesh`) "ECR_Ignore")
  ;;;[1 1 1] Play Dash Sound
  (bind _returnvalue (`FMODBlueprintStatics.PlayEvent2D` "/Game/FMOD/Events/Player/Dash.Dash"))
  (`FMODBlueprintStatics.EventInstancePlay` _returnvalue)
  (`FMODBlueprintStatics.EventInstanceRelease` _returnvalue))

(event `self.OnDashEnd`
  (bind _as_grim_game_mode (`self.As Grim Game Mode`))
  ;[1 0.433 0.3832 1 50] DASH
  ;;[1 1 1] DashFX
  (`|ExecutionSequence`
    (:`then_0`
      (`ActorComponent.SetActive` (`self.FX_Dash`) false false))
    (:`then_1`
      ;;[0 1 0.04734] Add 1 temp damage when dashing if player has Dash Training
      (if (`self.hasDashTraining`)
        (set `GrimGameMode.TileTempDashDamage` (+ (`GrimGameMode.TileTempDashDamage` _as_grim_game_mode) 1.0) _as_grim_game_mode)))))

(event `self.DashDamage.OnComponentBeginOverlap`
  (params (OverlappedComponent :type "PrimitiveComponent Object Reference") (OtherActor :type "Actor Object Reference") (OtherComp :type "PrimitiveComponent Object Reference") (OtherBodyIndex :type Integer) (bFromSweep :type Boolean) (SweepResult :type "HitResult Structure (by ref)"))
  ;[1 0.433 0.3832 1 50] DASH
  ;;[1 1 1] Dash Damage
  (bind _asbase_enemy (cast `BaseEnemy` OtherActor))
  (if (`self.hasDashDamage`)
    (if (`self.Dashing`)
      (bind _returnvalue (`GrimGameInstance.GetStat` (`self.As BP Grim Game Instance`) "DashDamage"))
      (bind _asbp_grim_game_mode (cast `/Game/Blueprints/GameEssentials/BP_GrimGameMode` (`GameplayStatics.GetGameMode`)))
      (`HealthComponent.TakeDamage` (`BaseEnemy.HealthComponent` _asbase_enemy) (+ _returnvalue (`GrimGameMode.TileTempDashDamage` _asbp_grim_game_mode)) false))))

(event `self.ReceiveDestroyed`)

(event `self.OnKick`
  (bind _kickcollider (`self.KickCollider`))
  (bind (_returnvalue_roll _returnvalue_pitch _returnvalue_yaw) (`KismetMathLibrary.BreakRotator` (`SceneComponent.K2_GetComponentRotation` _kickcollider)))
  (bind _returnvalue (`SceneComponent.K2_GetComponentLocation` _kickcollider))
  (bind (_returnvalue_roll_2 _returnvalue_pitch_2 _returnvalue_yaw_2) (`KismetMathLibrary.BreakRotator` (`SceneComponent.K2_GetComponentRotation` _kickcollider)))
  ;[1 1 1] Kick Function
  (`|ExecutionSequence`
    (:`then_0`
      (bind _outhit (`KismetSystemLibrary.SphereTraceSingle` :`Start` _returnvalue :`End` (+ _returnvalue (* (`KismetMathLibrary.GetForwardVector` (`KismetMathLibrary.MakeRotator` _returnvalue_roll_2 _returnvalue_pitch_2 (+ _returnvalue_yaw_2 0.0))) 200.0)) :`Radius` 1.0 :`TraceChannel` "TraceTypeQuery1" :`DrawDebugType` "ForDuration"))
      (bind (_bblockinghit _binitialoverlap _time _distance _location _impactpoint _normal _impactnormal _physmat _hitactor _hitcomponent) (`GameplayStatics.BreakHitResult` _outhit))
      (`/Engine/EditorBlueprintResources/StandardMacros.IsValid` _hitcomponent
        (:`Is Valid`
          (message `/Game/Blueprints/Player/BI_Kick.Kick` _hitactor)
          (`/Engine/EditorBlueprintResources/StandardMacros.IsValid` _hitcomponent
            (:`Is Valid`
              (`PrimitiveComponent.AddImpulse` _hitcomponent (* (`KismetMathLibrary.GetForwardVector` (`KismetMathLibrary.MakeRotator` _returnvalue_roll _returnvalue_pitch (+ _returnvalue_yaw 0.0))) 2500.0) "None" true)
              ;;[1 1 1] Play Kick Sound
              (bind _returnvalue_2 (`FMODBlueprintStatics.PlayEvent2D` "/Game/FMOD/Events/Player/Kick.Kick"))
              (`FMODBlueprintStatics.EventInstancePlay` _returnvalue_2)
              (`FMODBlueprintStatics.EventInstanceRelease` _returnvalue_2))))
        (:`Is Not Valid`
          (`KismetSystemLibrary.PrintString` "No object found for kick"))))
    (:`then_1`
      ;;[1 1 1] Play Kick in air sound
      (bind _returnvalue_3 (`FMODBlueprintStatics.PlayEvent2D` "/Game/FMOD/Events/Player/KickInAir.KickInAir"))
      (`FMODBlueprintStatics.EventInstancePlay` _returnvalue_3)
      (`FMODBlueprintStatics.EventInstanceRelease` _returnvalue_3))))

(event `self.OnAttack`
  ;[1 1 1] VFX Slash Attack
)

(event `self.OnReturnScythe`
  (`SceneComponent.SetVisibility` (`self.SkeletalMesh`) true true)
  (`self.SetIsCasting` false))

(event `AnimAttackNotify`
  (params (Combo :type "EPlayerStatType Enum" :default "MovementSpeed"))
  (bind _skeletalmesh (`self.SkeletalMesh`))
  ;[1 1 1] Attack Combo Collision enabling - Called from AnimNotify in ComboMontage
  (set `self.Stat Type` Combo)
  (`KismetArrayLibrary.Array_Clear` (`self.Other Actor`))
  (`PrimitiveComponent.SetCollisionResponseToAllChannels` _skeletalmesh "ECR_Overlap")
  (`PrimitiveComponent.SetCollisionEnabled` _skeletalmesh "NoCollision")
  (`PrimitiveComponent.SetCollisionEnabled` _skeletalmesh "QueryAndPhysics"))

(event `RemoveCollision`
  ;[1 1 1] Attack Combo Collision enabling - Called from AnimNotify in ComboMontage
  (`PrimitiveComponent.SetCollisionResponseToAllChannels` (`self.SkeletalMesh`) "ECR_Ignore"))

(event `HideScythe`
  ;[1 0.2546 0.9624 1 35] Schyte Attack
  (`SceneComponent.SetVisibility` (`self.SkeletalMesh`) false false))

(event `self.SkeletalMesh.OnComponentBeginOverlap`
  (params (OverlappedComponent :type "PrimitiveComponent Object Reference") (OtherActor :type "Actor Object Reference") (OtherComp :type "PrimitiveComponent Object Reference") (OtherBodyIndex :type Integer) (bFromSweep :type Boolean) (SweepResult :type "HitResult Structure (by ref)"))
  (bind _returnvalue (`self.GetComponentByClass` OtherActor "/Script/GP3Team3.HealthComponent"))
  (bind _as_bp_grim_game_instance (`self.As BP Grim Game Instance`))
  (bind _as_grim_game_mode (`self.As Grim Game Mode`))
  (bind _tiletempdamage (`GrimGameMode.TileTempDamage` _as_grim_game_mode))
  ;[1 0.2546 0.9624 1 35] Schyte Attack
  (`|ExecutionSequence`
    (:`then_0`
      (set `self.critRandomizer` (`KismetMathLibrary.RandomFloatInRange` 0.0 100.0)))
    (:`then_1`
      (if (== OtherActor self)
        _
        (elif (not (`KismetArrayLibrary.Array_Contains` (`self.Other Actor`) OtherActor))
          (`/Engine/EditorBlueprintResources/StandardMacros.IsValid` _returnvalue
            (:`Is Valid`
              (bind _returnvalue_2 (`GrimGameInstance.GetStat` _as_bp_grim_game_instance (`self.Stat Type`)))
              (bind _returnvalue_3 (`GrimGameInstance.GetStat` _as_bp_grim_game_instance "BaseDamageMultiplier"))
              (bind _returnvalue_4 (`GrimGameInstance.GetStat` _as_bp_grim_game_instance "CritChance"))
              (bind _returnvalue_5 (`GrimGameInstance.GetStat` _as_bp_grim_game_instance "CritDamage"))
              (if (`self.hasPOG`)
                (bind _returnvalue_6 (<= (`self.critRandomizer`) _returnvalue_4))
                (if _returnvalue_6
                  (bind _returnvalue_7 (* _returnvalue_3 _returnvalue_2))
                  (bind _returnvalue_8 (+ _tiletempdamage (+ (* (`KismetMathLibrary.Conv_IntToDouble` (`GrimGameMode.LevelCurrency` _as_grim_game_mode)) 0.05) _returnvalue_7)))
                  (`HealthComponent.TakeDamage` _returnvalue (+ _returnvalue_8 _returnvalue_5) true)
                  ;;[1 1 1] Play Fmod Crit Sound
                  (bind _returnvalue_9 (`FMODBlueprintStatics.PlayEvent2D` "/Game/FMOD/Events/Player/Crit.Crit"))
                  (`FMODBlueprintStatics.EventInstancePlay` _returnvalue_9)
                  (`FMODBlueprintStatics.EventInstanceRelease` _returnvalue_9)
                  (else
                    (`HealthComponent.TakeDamage` _returnvalue _returnvalue_8 false)))
                (elif _returnvalue_6
                  (bind _returnvalue_10 (+ _tiletempdamage _returnvalue_7))
                  (`HealthComponent.TakeDamage` _returnvalue (+ _returnvalue_10 _returnvalue_5) true)
                  ;;[1 1 1] Play Fmod Crit Sound
                  (bind _returnvalue_11 (`FMODBlueprintStatics.PlayEvent2D` "/Game/FMOD/Events/Player/Crit.Crit"))
                  (`FMODBlueprintStatics.EventInstancePlay` _returnvalue_11)
                  (`FMODBlueprintStatics.EventInstanceRelease` _returnvalue_11)
                  (else
                    (`HealthComponent.TakeDamage` _returnvalue _returnvalue_10 false))))
              (`KismetArrayLibrary.Array_Add` (`self.Other Actor`) OtherActor))))))))

(event `self.AuraComponent.OnEnemyDamaged`
  (bind _as_grim_game_mode (`self.As Grim Game Mode`))
  ;[1 0.9105 0.7832 1 40] Aura
  ;;[0.2451 0.01415 1 1 20] Add 1 temp aura dmg per enemy hit (if player has Worsening Weather)
  (if (`self.hasWorseningWeather`)
    (set `GrimGameMode.TileTempAuraDamage` (+ (`GrimGameMode.TileTempAuraDamage` _as_grim_game_mode) 1.0) _as_grim_game_mode)))

(event `self.AuraComponent.OnAuraGet`
  ;[1 0.9105 0.7832 1 40] Aura
  (`SceneComponent.SetVisibility` (`self.NS_AuraVFX`) true false))

(event `self.HealthComponent.OnHit`
  (params (DamageAmount :type "Float (single-precision)") (CritDamage :type Boolean))
  (bind _as_grim_game_mode (`self.As Grim Game Mode`))
  ;[1 0.4612 0.3914 1 35] ON GETTING HIT
  (`|ExecutionSequence`
    (:`then_0`
      ;[1 0.4311 0 1 25] Lose money on damage taken
      (bind _asbp_grim_game_mode (cast `/Game/Blueprints/GameEssentials/BP_GrimGameMode` (`GameplayStatics.GetGameMode`)))
      (if (> (`GrimGameMode.LevelCurrency` _asbp_grim_game_mode) 0)
        (if (not (`self.hasPennyPinch`))
          (`GrimGameMode.SpendLevelCurrency` _asbp_grim_game_mode 1))))
    (:`then_1`
      ;[0.8389 0 1 1 30] Add 5 temp damage on getting hit (if Badge of Wrath is gotten)
      (if (`self.hasBOW`)
        (set `GrimGameMode.TileTempDamage` (+ (`GrimGameMode.TileTempDamage` _as_grim_game_mode) 5.0) _as_grim_game_mode)))
    (:`then_2`
      ;[1 1 1] Play Player Hurt Sound
      (bind _returnvalue (`FMODBlueprintStatics.PlayEvent2D` "/Game/FMOD/Events/Player/Hurt.Hurt"))
      (`FMODBlueprintStatics.EventInstancePlay` _returnvalue)
      (`FMODBlueprintStatics.EventInstanceRelease` _returnvalue))
    (:`then_3`
      ;[1 1 1] Hurt UI
      (bind _returnvalue_2 (`|GenericCreateObject` "/Game/Blueprints/UI/WB_Hurt.WB_Hurt_C"))
      (`UserWidget.AddToViewport` _returnvalue_2 0))
    (:`then_4`
      ;[1 1 1] FMOD Turn on off Low Health filter
      (bind _asbp_grim_game_mode_2 (cast `/Game/Blueprints/GameEssentials/BP_GrimGameMode` (`GameplayStatics.GetGameMode`)))
      (if (<= (`HealthComponent.CurrentHealth` (`self.HealthComponent`)) 20.0)
        (`/Game/Blueprints/GameEssentials/BP_GrimGameMode.TurnOnLowHealth` _asbp_grim_game_mode_2 false)
        (else
          (`/Game/Blueprints/GameEssentials/BP_GrimGameMode.TurnOffLowHealth` _asbp_grim_game_mode_2 false))))))

(event `Key|Escape` :paused true
  (params (Key :type "Key Structure"))
  (bind _returnvalue (`GameplayStatics.GetPlayerController` 0))
  (:`Pressed`
    (if (`self.isPaused`) :!label _label
      (set `self.isPaused` false)
      (bind _returnvalue_2 (`|GenericCreateObject` _returnvalue "/Game/Blueprints/UI/WB_PauseScreen.WB_PauseScreen_C"))
      (bind _output_get (set `self.PauseMenuWidget` _returnvalue_2))
      (`UserWidget.AddToViewport` _output_get 0)
      (`WidgetBlueprintLibrary.SetInputMode_GameAndUIEx` _returnvalue (`self.PauseMenuWidget`))
      (set `PlayerController.bShowMouseCursor` true (`GameplayStatics.GetPlayerController` 0))
      (`GameplayStatics.SetGamePaused` true)
      (else
        (set `self.isPaused` true)
        (`Widget.RemoveFromParent` (`self.PauseMenuWidget`))
        (`GameplayStatics.SetGamePaused` false)
        (`WidgetBlueprintLibrary.SetInputMode_GameOnly` _returnvalue)
        (set `PlayerController.bShowMouseCursor` false (`GameplayStatics.GetPlayerController` 0))))))

(event `Key|Z` :paused true
  (params (Key :type "Key Structure"))
  (:`Pressed`
    (goto _label)))

(fn `UserConstructionScript`)