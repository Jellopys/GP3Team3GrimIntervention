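; Thrown scythe projectile for the player's scythe toss, damaging actors with a health component that it overlaps.
; Cast, apex and return events toggle the sphere's collision, manage the throw sound and clear the player's casting state on return.
; Damage combines game-instance toss damage and base multiplier stats.
; A hit list prevents repeat hits and is cleared at cast and apex, so targets can be hit on each leg.
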(event `self.ReceiveBeginPlay`
  (bind _asbp_grim_game_instance (cast `/Game/Blueprints/GameEssentials/BP_GrimGameInstance` (`GameplayStatics.GetGameInstance`)))
  (set `self.As BP Grim Game Instance` _asbp_grim_game_instance)
  (bind _asbp_player_character (cast `/Game/Blueprints/Player/BP_PlayerCharacter` (`GameplayStatics.GetPlayerPawn` 0)))
  (set `self.As BP Player Character` _asbp_player_character))

(event `self.OnScytheCast`
  (`PrimitiveComponent.SetCollisionResponseToAllChannels` (`self.Sphere`) "ECR_Overlap")
  (`KismetArrayLibrary.Array_Clear` (`self.Other Actor`))
  (bind _returnvalue (`FMODBlueprintStatics.PlayEvent2D` "/Game/FMOD/Events/Player/MeleeAttackThrow.MeleeAttackThrow" false))
  (bind _output_get (set `self.MeleeThrowSound` _returnvalue))
  (`FMODBlueprintStatics.EventInstancePlay` _returnvalue)
  (`FMODBlueprintStatics.EventInstanceRelease` _returnvalue))

(event `self.OnScytheReturn`
  (`PrimitiveComponent.SetCollisionResponseToAllChannels` (`self.Sphere`) "ECR_Ignore")
  (`PlayerCharacter.SetIsCasting` (`self.As BP Player Character`) false)
  (`FMODBlueprintStatics.EventInstanceStop` (stale `self.OnScytheCast` _output_get)))

(event `self.OnScytheReachApex`
  (`KismetArrayLibrary.Array_Clear` (`self.Other Actor`)))

(event `self.Sphere.OnComponentBeginOverlap`
  (params (OverlappedComponent :type "PrimitiveComponent Object Reference") (OtherActor :type "Actor Object Reference") (OtherComp :type "PrimitiveComponent Object Reference") (OtherBodyIndex :type Integer) (bFromSweep :type Boolean) (SweepResult :type "HitResult Structure (by ref)"))
  (bind _returnvalue (`self.GetComponentByClass` OtherActor "/Script/GP3Team3.HealthComponent"))
  (bind _as_bp_grim_game_instance (`self.As BP Grim Game Instance`))
  (if (== OtherActor (`self.As BP Player Character`))
    _
    (elif (not (`KismetArrayLibrary.Array_Contains` (`self.Other Actor`) OtherActor))
      (`/Engine/EditorBlueprintResources/StandardMacros.IsValid` _returnvalue
        (:`Is Valid`
          (bind _returnvalue_2 (`GrimGameInstance.GetStat` _as_bp_grim_game_instance "BaseDamageMultiplier"))
          (bind _returnvalue_3 (`GrimGameInstance.GetStat` _as_bp_grim_game_instance "ScytheTossDamage"))
          (`HealthComponent.TakeDamage` _returnvalue (* _returnvalue_3 _returnvalue_2) false)
          (`KismetArrayLibrary.Array_Add` (`self.Other Actor`) OtherActor))))))

(fn `UserConstructionScript`)