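; BP_GrimGameMode is the game mode that runs level audio, the minimap overlay and boss room progression.
; BeginPlay creates the hidden, Tab-toggled minimap and starts FMOD music, atmosphere and low-health events, while later events handle boss music, wall sounds and low-health parameters.
; Tile clears update the minimap counter and chest-spacing count, opening boss tiles with a popup once a threshold is reached.
; It also resets temporary damage stats and shows the win screen when walls drop.
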(event `Play Boss Music`
  ;[1 1 1] FMOD Boss music
  (bind _returnvalue (`FMODBlueprintStatics.PlayEvent2D` "/Game/FMOD/Events/Music/Boss.Boss"))
  (bind _output_get (set `self.BossMusic` _returnvalue))
  (`FMODBlueprintStatics.EventInstancePlay` _output_get)
  (`FMODBlueprintStatics.EventInstanceRelease` _output_get))

(event `OnTabPressed`
  ;[0.7508 1 0.5813 1 32] Create MiniMap Overlay
  (switch `ESlateVisibility` (`Widget.GetVisibility` (stale `self.ReceiveBeginPlay` _returnvalue))
    (:`Visible`
      (`Widget.SetVisibility` (stale `self.ReceiveBeginPlay` _returnvalue) "Hidden"))
    (:`Hidden`
      (`Widget.SetVisibility` (stale `self.ReceiveBeginPlay` _returnvalue) "Visible"))))

(event `self.ResetTempStats`
  ;[0.5512 0.8369 1 1 25] Reset temp stat event
  (set `self.TileTempDamage` 0.0)
  (set `self.TileTempAuraDamage` 0.0)
  (set `self.TileTempDashDamage` 0.0))

(event `self.ReceiveBeginPlay`
  ;[0.7508 1 0.5813 1 32] Create MiniMap Overlay
  (`|ExecutionSequence`
    (:`then_0`
      (bind _returnvalue (`|CreateWidget` "/Game/UI/MiniMap/UW_MiniMapOverlay.UW_MiniMapOverlay_C" (`GameplayStatics.GetPlayerController` 0)))
      (`UserWidget.AddToPlayerScreen` _returnvalue 1000)
      (`Widget.SetVisibility` _returnvalue "Hidden"))
    (:`then_1`
      ;[1 1 1] FMOD Level music
      (bind _returnvalue_2 (`FMODBlueprintStatics.PlayEvent2D` "/Game/FMOD/Events/Music/Level.Level"))
      (bind _output_get (set `self.LevelMusic` _returnvalue_2))
      (`FMODBlueprintStatics.EventInstancePlay` _output_get)
      (`FMODBlueprintStatics.EventInstanceRelease` _output_get))
    (:`then_2`
      ;[1 1 1] FMOD Atmosphere sounds
      (bind _returnvalue_3 (`FMODBlueprintStatics.PlayEvent2D` "/Game/FMOD/Events/Atmosphere/Atmosphere.Atmosphere"))
      (bind _output_get_2 (set `self.Atmosphere` _returnvalue_3))
      (`FMODBlueprintStatics.EventInstancePlay` _output_get_2)
      (`FMODBlueprintStatics.EventInstanceRelease` _output_get_2))
    (:`then_3`
      ;[1 1 1] FMOD Low Health music
      (bind _returnvalue_4 (`FMODBlueprintStatics.PlayEvent2D` "/Game/FMOD/Events/Music/LowHealthMusic.LowHealthMusic"))
      (bind _output_get_3 (set `self.LowHealthMusic` _returnvalue_4))
      (`FMODBlueprintStatics.EventInstancePlay` _output_get_3)
      (`FMODBlueprintStatics.EventInstanceRelease` _output_get_3))
    (:`then_4`
      ;[1 1 1] FMOD Play Low Health Event
      (bind _returnvalue_5 (`FMODBlueprintStatics.PlayEvent2D` "/Game/FMOD/Events/LowHealthEvent.LowHealthEvent"))
      (bind _output_get_4 (set `self.LowHealthEvent` _returnvalue_5))
      (`FMODBlueprintStatics.EventInstancePlay` _output_get_4))))

(event `TurnOnLowHealth`
  (params (Condition :type Boolean))
  ;[1 1 1] Set FMOD Parameter LowHealth to 0
  (`FMODBlueprintStatics.EventInstanceSetParameter` (stale `self.ReceiveBeginPlay` _output_get_4) "VeryLowHealth" (`self.LowHealth`)))

(event `self.OnTileExplored`)

(event `TurnOffLowHealth`
  (params (Condition :type Boolean))
  ;[1 1 1] Set FMOD Parameter LowHealth to 1
  (`FMODBlueprintStatics.EventInstanceSetParameter` (stale `self.ReceiveBeginPlay` _output_get_4) "VeryLowHealth" (`self.NormalHealth`)))

(event `self.OnTileCleared`
  (bind _tilescleared (`self.TilesCleared`))
  (`|ExecutionSequence`
    (:`then_0`
      ;[0.3924 1 0.1458 1 30] Set MiniMap Cleared Text
      (`TextBlock.SetText` (`/Game/UI/MiniMap/UW_MiniMapOverlay.MiniMapClearCounterTxt` (stale `self.ReceiveBeginPlay` _returnvalue)) (`KismetTextLibrary.Conv_StringToText` (`KismetStringLibrary.Concat_StrStr` (`KismetStringLibrary.Conv_IntToString` _tilescleared) " / 100 Cleared"))))
    (:`then_1`
      ;[1 0.4323 0.467 1 30] Check to Open Boss Room
      (if (>= _tilescleared 15)
        (if (not (`self.BossRoomIsOpen`))
          (`KismetSystemLibrary.Delay` 3.5)
          (bind _returnvalue (`|GenericCreateObject` "/Game/Blueprints/UI/WB_BossOpened.WB_BossOpened_C"))
          (`UserWidget.AddToViewport` _returnvalue 0)
          (bind _outactors (`GameplayStatics.GetAllActorsOfClass` "/Game/Blueprints/Rooms/Boss/BP_BossTile.BP_BossTile_C"))
          (for _array_element _outactors
            (`BossTile.OpenBossRoom` _array_element)
            (set `self.BossRoomIsOpen` true)
            ;[1 1 1] Play FMOD BossRoomOpen - 15 Tiles
            (bind _returnvalue_2 (`FMODBlueprintStatics.PlayEvent2D` "/Game/FMOD/Events/Level/BossRoomOpen.BossRoomOpen"))
            (`FMODBlueprintStatics.EventInstancePlay` _returnvalue_2)
            (`FMODBlueprintStatics.EventInstanceRelease` _returnvalue_2)))))
    (:`then_2`
      ;[0.7021 0.7342 1 1 25] Add To LastChest Counter
      (set `self.roomsSinceChest` (+ (`self.roomsSinceChest`) 1)))))

(event `self.OnWallsUp`
  ;[1 0.5639 0.8558 1 40] ON WALLS UP & DOWN
  ;;[1 1 1] Play Event Fight Sound (Wall)
  (bind _returnvalue (`FMODBlueprintStatics.PlayEvent2D` "/Game/FMOD/Events/Level/Wall.Wall"))
  (bind _output_get (set `self.Wall` _returnvalue))
  (`FMODBlueprintStatics.EventInstancePlay` _output_get)
  (`FMODBlueprintStatics.EventInstanceRelease` _output_get))

(event `self.OnWallsDown`
  ;[1 0.5639 0.8558 1 40] ON WALLS UP & DOWN
  (`|ExecutionSequence`
    (:`then_0`
      ;;[1 1 1] Set FMOD Parameter to 1. So sound jumps to end. Set back to 0.
      (`FMODBlueprintStatics.EventInstanceSetParameter` (stale `self.OnWallsUp` _output_get) "End" (`self.pitch`)))
    (:`then_1`
      (bind _returnvalue (`|GenericCreateObject` "/Game/Blueprints/UI/WB_WinScreen.WB_WinScreen_C"))
      (`UserWidget.AddToViewport` _returnvalue 0))))

(fn `UserConstructionScript`)