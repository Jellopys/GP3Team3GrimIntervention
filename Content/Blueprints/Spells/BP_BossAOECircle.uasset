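; Boss area-of-effect circle spell that deals a delayed burst of damage to the player.
; On BeginPlay it caches the player character and starts a timer that briefly switches the Sphere to overlap all channels, then disables it and destroys the actor.
; Overlaps with the player apply DMG through HealthComponent, with a hit-list check to prevent repeat damage.
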(event `self.ReceiveBeginPlay`
  (bind _asbp_player_character (cast `/Game/Blueprints/Player/BP_PlayerCharacter` (`GameplayStatics.GetPlayerPawn` 0)))
  (set `self.As BP Player Character` _asbp_player_character)
  (`KismetSystemLibrary.K2_SetTimerDelegate` (delegate `AddCollision`) 1.2))

(event `AddCollision`
  (`PrimitiveComponent.SetCollisionResponseToAllChannels` (`self.Sphere`) "ECR_Overlap")
  (`KismetSystemLibrary.Delay` 0.1)
  (`PrimitiveComponent.SetCollisionResponseToAllChannels` (`self.Sphere`) "ECR_Ignore")
  (`KismetSystemLibrary.Delay` 0.3)
  (`self.K2_DestroyActor`))

(event `self.Sphere.OnComponentBeginOverlap`
  (params (OverlappedComponent :type "PrimitiveComponent Object Reference") (OtherActor :type "Actor Object Reference") (OtherComp :type "PrimitiveComponent Object Reference") (OtherBodyIndex :type Integer) (bFromSweep :type Boolean) (SweepResult :type "HitResult Structure (by ref)"))
  (bind _returnvalue (`self.GetComponentByClass` OtherActor "/Script/GP3Team3.HealthComponent"))
  (if (== OtherActor (`self.As BP Player Character`))
    (if (not (`KismetArrayLibrary.Array_Contains` (`self.Other Actor`) OtherActor))
      (`/Engine/EditorBlueprintResources/StandardMacros.IsValid` _returnvalue
        (:`Is Valid`
          (`HealthComponent.TakeDamage` _returnvalue (`self.DMG`) false)
          (`KismetArrayLibrary.Array_Add` (`self.Other Actor`) OtherActor))))))

(fn `UserConstructionScript`)