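; Power-up chest that appears as treasure on the minimap and opens when the player character overlaps its trigger box.
; On BeginPlay it registers with the game mode's minimap widget; OpenChest is called here but defined elsewhere.
; The open event switches to UI-only input and freezes the player.
; The close event removes the icon, plays a leaving animation, restores game input, re-enables movement unless the player is dead, then destroys the chest after a delay.
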(event `self.ReceiveBeginPlay`
  ;[1 1 1] Treasure on map
  (bind _asbp_grim_game_mode (cast `/Game/Blueprints/GameEssentials/BP_GrimGameMode` (`GameplayStatics.GetGameMode`)))
  (bind _minimapwidget (`/Game/Blueprints/GameEssentials/BP_GrimGameMode.MiniMapWidget` _asbp_grim_game_mode))
  (set `self.Mini Map Widget` _minimapwidget)
  (`/Game/UI/MiniMap/UW_MiniMapWidget.AddTreasure` _minimapwidget self)
  (bind _asbp_player_character (cast `/Game/Blueprints/Player/BP_PlayerCharacter` (`GameplayStatics.GetPlayerPawn` 0)))
  (set `self.As BP Player Character` _asbp_player_character))

(event `self.TriggerBox.OnComponentBeginOverlap`
  (params (OverlappedComponent :type "PrimitiveComponent Object Reference") (OtherActor :type "Actor Object Reference") (OtherComp :type "PrimitiveComponent Object Reference") (OtherBodyIndex :type Integer) (bFromSweep :type Boolean) (SweepResult :type "HitResult Structure (by ref)"))
  (if (== OtherActor (`self.As BP Player Character`))
    (`self.OpenChest`)))

(event `self.OnChestOpen`
  (`WidgetBlueprintLibrary.SetInputMode_UIOnlyEx` (`GameplayStatics.GetPlayerController` 0) null)
  (`PlayerCharacter.SetCanMove` (`self.As BP Player Character`) false))

(event `self.OnChestClose`
  (bind _returnvalue (`GameplayStatics.GetPlayerController` 0))
  (bind _as_bp_player_character (`self.As BP Player Character`))
  (`/Game/UI/MiniMap/UW_MiniMapWidget.RemoveTreasure` (`self.Mini Map Widget`) (`self.TreasureIconRef`))
  (`SkeletalMeshComponent.PlayAnimation` (`self.ChestMesh`) "/Game/Environment/Animated_props/chestLeaving.chestLeaving" false)
  (if (`HealthComponent.bIsDead` (`PlayerCharacter.HealthComponent` _as_bp_player_character))
    (`WidgetBlueprintLibrary.SetInputMode_GameOnly` _returnvalue)
    (else
      (`WidgetBlueprintLibrary.SetInputMode_GameOnly` _returnvalue)
      (`PlayerCharacter.SetCanMove` _as_bp_player_character true)))
  (`KismetSystemLibrary.Delay` 3.0)
  (`self.K2_DestroyActor`))

(fn `UserConstructionScript`)