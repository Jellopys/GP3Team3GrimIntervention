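; BP_LootSpawner is a hidden marker actor that spawns either a power-up chest or scattered coins when its OnLootSpawned event fires.
; A chest roll uses a base chance boosted by GameInstance luck upgrades, with a GameMode room counter guaranteeing a chest after three misses.
; Chest spawns reset that counter, while failed rolls increment it and drop a random, luck-scaled number of coins around the spawner.
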(event `self.ReceiveBeginPlay`
  ;[1 0.1557 0.1855 1 30] BEGIN PLAY
  (`SceneComponent.SetVisibility` (`self.Cube`) false false)
  (bind _asbp_grim_game_mode (cast `/Game/Blueprints/GameEssentials/BP_GrimGameMode` (`GameplayStatics.GetGameMode`)))
  (set `self.As BP Grim Game Mode` _asbp_grim_game_mode)
  (bind _asbp_grim_game_instance (cast `/Game/Blueprints/GameEssentials/BP_GrimGameInstance` (`GameplayStatics.GetGameInstance`)))
  (set `self.As BP Grim Game Instance` _asbp_grim_game_instance))

(event `self.OnLootSpawned`
  (bind (_returnvalue_x _returnvalue_y _returnvalue_z) (`KismetMathLibrary.BreakVector` (`self.K2_GetActorLocation`)))
  (bind _as_bp_grim_game_mode (`self.As BP Grim Game Mode`))
  (bind _returnvalue (`KismetMathLibrary.Conv_VectorToTransform` (`self.K2_GetActorLocation`)))
  (bind _roomssincechest (`/Game/Blueprints/GameEssentials/BP_GrimGameMode.roomsSinceChest` _as_bp_grim_game_mode))
  (bind _luckupgrades (`GrimGameInstance.LuckUpgrades` (`self.As BP Grim Game Instance`)))
  ;[1 0.7659 0.2327 1 45] SPAWN LOOT
  (`KismetSystemLibrary.PrintString` "Loot spawning" true true (struct :`R` 1.0 :`B` 0.003789 :`A` 1.0) 5.0)
  (if (>= _roomssincechest 3)
    (set `/Game/Blueprints/GameEssentials/BP_GrimGameMode.roomsSinceChest` 0 _as_bp_grim_game_mode :!label _label)
    (`KismetSystemLibrary.PrintString` (`KismetStringLibrary.Concat_StrStr` "Trying To Spawn Chest at: " (`KismetStringLibrary.Conv_TransformToString` _returnvalue)) true true (struct :`G` 0.66 :`B` 1.0 :`A` 1.0) 5.0)
    (bind _returnvalue_2 (`|SpawnActorFromClass` "/Game/Blueprints/PowerUps/BP_PowerUpChest.BP_PowerUpChest_C" _returnvalue "AlwaysSpawn" "OverrideRootScale" null null))
    (`/Engine/EditorBlueprintResources/StandardMacros.IsValid` _returnvalue_2
      (:`Is Valid`
        (`KismetSystemLibrary.PrintString` "Spawned Chest" true true (struct :`R` 1.0 :`B` 0.003789 :`A` 1.0) 5.0)))
    (elif (<= (`KismetMathLibrary.RandomFloatInRange` 0.0 100.0) (+ (`self.ChestPercentChance`) (* _luckupgrades 5)))
      (goto _label)
      (else
        (set `/Game/Blueprints/GameEssentials/BP_GrimGameMode.roomsSinceChest` (+ _roomssincechest 1) _as_bp_grim_game_mode)
        (for _ (range 1 (+ (`KismetMathLibrary.RandomIntegerInRange` (+ _luckupgrades 1) (+ _luckupgrades 3)) 1))
          (bind _returnvalue_3 (`|SpawnActorFromClass` "/Game/Blueprints/Items/BP_TheCoinPickup.BP_TheCoinPickup_C" (`KismetMathLibrary.Conv_VectorToTransform` (`KismetMathLibrary.MakeVector` (+ _returnvalue_x (`KismetMathLibrary.RandomFloatInRange` -50.0 50.0)) (+ _returnvalue_y (`KismetMathLibrary.RandomFloatInRange` -50.0 50.0)) _returnvalue_z)) "AlwaysSpawn" "OverrideRootScale" null null))
          (`/Engine/EditorBlueprintResources/StandardMacros.IsValid` _returnvalue_3
            (:`Is Valid`
              (`KismetSystemLibrary.PrintString` "Spawned Coin" true true (struct :`R` 1.0 :`B` 0.003789 :`A` 1.0) 5.0))))))))

(fn `UserConstructionScript`)