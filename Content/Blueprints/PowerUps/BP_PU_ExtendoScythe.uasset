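; Power-up Blueprint for the Extendo Scythe, meant to trade combo damage for faster attacks (+50% speed, -50% damage).
; When gotten, it reads attack speed and first, second and third combo damage from the GameInstance through small getter functions wrapping GetStat.
; It passes the scaled values back through GameInstance UpgradeStat, one call per stat type.
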(event `self.OnPowerUpGotten`
  (bind _gameinstance (`self.GameInstance`))
  ;[0.633 0.9601 1 1 30] +50% attack spd & -50% dmg
  (bind _returnvalue (`GrimGameInstance.GetStat` _gameinstance "AttackSpeed"))
  (`GrimGameInstance.UpgradeStat` _gameinstance (* _returnvalue 1.5) "AttackSpeed")
  (bind _returnvalue_2 (`GrimGameInstance.GetStat` _gameinstance "FirstComboDamage"))
  (`GrimGameInstance.UpgradeStat` _gameinstance (/ _returnvalue_2 2.0) "FirstComboDamage")
  (bind _returnvalue_3 (`GrimGameInstance.GetStat` _gameinstance "SecondComboDamage"))
  (`GrimGameInstance.UpgradeStat` _gameinstance (/ _returnvalue_3 2.0) "SecondComboDamage")
  (bind _returnvalue_4 (`GrimGameInstance.GetStat` _gameinstance "ThirdComboDamage"))
  (`GrimGameInstance.UpgradeStat` _gameinstance (/ _returnvalue_4 2.0) "ThirdComboDamage"))