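; BP_KickExplosive is an environment prop that explodes when kicked or when its Health runs out.
; Kick turns on physics for the Cylinder, then after a short fixed delay joins the death path.
; Explosive damage feeds the Health component unless the prop is already Broken.
; The death path sets Broken, spawns BP_Explosive at the Cylinder's current location and destroys the actor.
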(event `self.Health.OnDeath`
  ;[1 1 1] Push and spawn coins + particles on kick
  (set `self.Broken` true :!label _label)
  (`|SpawnActorFromClass` "/Game/Blueprints/Environment/BP_Explosive.BP_Explosive_C" (`KismetMathLibrary.Conv_VectorToTransform` (`SceneComponent.K2_GetComponentLocation` (`self.Cylinder`))) "AdjustIfPossibleButAlwaysSpawn" "OverrideRootScale" null null)
  (`self.K2_DestroyActor`))

(event `/Game/Blueprints/Player/BI_Kick.Kick`
  ;[1 1 1] Push and spawn coins + particles on kick
  (set `self.doKick` true)
  (`PrimitiveComponent.SetSimulatePhysics` (`self.Cylinder`) true)
  (`KismetSystemLibrary.Delay` 0.6)
  (goto _label))

(event `/Game/Blueprints/Interfaces/BI_ExplosiveDamage.ExplosiveDamage`
  (if (not (`self.Broken`))
    (`HealthComponent.TakeDamage` (`self.Health`) 1.0 false)))

(fn `UserConstructionScript`)