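; BP_Explosive is a short-lived explosion actor that detonates as soon as it begins play.
; BeginPlay activates the explosion VFX and plays the Explosion audio event at its location.
; The Collision component sends ExplosiveDamageMessage to any valid overlapping actor, leaving the damage response to the receiver.
; Collision is destroyed after a brief damage window, and the actor destroys itself a second later.
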(event `self.ReceiveBeginPlay`
  (`ActorComponent.Activate` (`self.ExplosionVFX`) false)
  (`FMODBlueprintStatics.PlayEventAtLocation` "/Game/FMOD/Events/Objects/Explosion.Explosion" (`KismetMathLibrary.Conv_VectorToTransform` (`SceneComponent.K2_GetComponentLocation` (`self.ExplosionVFX`))))
  (`KismetSystemLibrary.Delay` 0.75)
  (`ActorComponent.K2_DestroyComponent` (`self.Collision`))
  (`KismetSystemLibrary.Delay` 1.0)
  (`self.K2_DestroyActor`))

(event `self.Collision.OnComponentBeginOverlap`
  (params (OverlappedComponent :type "PrimitiveComponent Object Reference") (OtherActor :type "Actor Object Reference") (OtherComp :type "PrimitiveComponent Object Reference") (OtherBodyIndex :type Integer) (bFromSweep :type Boolean) (SweepResult :type "HitResult Structure (by ref)"))
  (`/Engine/EditorBlueprintResources/StandardMacros.IsValid` OtherActor
    (:`Is Valid`
      (message `/Game/Blueprints/Interfaces/BI_ExplosiveDamage.ExplosiveDamage` OtherActor))))

(fn `UserConstructionScript`)