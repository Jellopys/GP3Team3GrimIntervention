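; BP_BreakableChair is a destructible chair prop that breaks when kicked or when its Health component reports death.
; Explosive damage feeds into Health, while a kick skips it and runs the break logic directly.
; Breaking rolls a small chance for a coin pickup, then a health pickup if that fails, spawns the reused BP_UrnBreak effect, plays a furniture-break sound and destroys the actor.
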(event `self.Health.OnDeath`
  (bind _returnvalue (`KismetMathLibrary.Conv_VectorToTransform` (`SceneComponent.K2_GetComponentLocation` (`self.StaticMesh`))))
  ;[1 1 1] Push and spawn coins + particles on kick
  (`|ExecutionSequence` :!label _label
    (:`then_0`
      (if (<= (`KismetMathLibrary.RandomFloatInRange` 0.0 100.0) 10.0)
        (`|SpawnActorFromClass` "/Game/Blueprints/Items/BP_TheCoinPickup.BP_TheCoinPickup_C" _returnvalue "AdjustIfPossibleButAlwaysSpawn" "OverrideRootScale" null null)
        (elif (<= (`KismetMathLibrary.RandomFloatInRange` 0.0 100.0) 10.0)
          (`|SpawnActorFromClass` "/Game/Blueprints/Items/BP_HealthPickup.BP_HealthPickup_C" _returnvalue "AdjustIfPossibleButAlwaysSpawn" "OverrideRootScale" null null))))
    (:`then_1`
      (`|SpawnActorFromClass` "/Game/Blueprints/Environment/BP_UrnBreak.BP_UrnBreak_C" _returnvalue "AdjustIfPossibleButAlwaysSpawn" "OverrideRootScale" null null)
      (`FMODBlueprintStatics.PlayEvent2D` "/Game/FMOD/Events/Objects/FurnitureBreak.FurnitureBreak")
      (`FMODBlueprintStatics.EventInstancePlay` (struct))
      (`FMODBlueprintStatics.EventInstanceRelease` (struct))
      (`self.K2_DestroyActor`))))

(event `/Game/Blueprints/Player/BI_Kick.Kick`
  ;[1 1 1] Push and spawn coins + particles on kick
  (goto _label))

(event `/Game/Blueprints/Interfaces/BI_ExplosiveDamage.ExplosiveDamage`
  (`HealthComponent.TakeDamage` (`self.Health`) 1.0 false))

(fn `UserConstructionScript`)