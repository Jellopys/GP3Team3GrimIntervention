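; Soul orb pickup that homes in on the player and restores health on collection.
; Player overlap with the Radius starts a timeline that moves the orb via VInterpTo, using the timeline's value as delta time.
; Once any overlap arms it, Tick checks player distance, then grants health, plays an FMOD sound and destroys the actor.
; It then asks the Grim game mode to turn off the low-health audio filter if health is above the threshold.
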(event `self.ReceiveBeginPlay`
  (bind _asbp_player_character (cast `/Game/Blueprints/Player/BP_PlayerCharacter` (`GameplayStatics.GetPlayerPawn` 0)))
  (set `self.PlayerRef` _asbp_player_character))

(event `self.radius.OnComponentBeginOverlap`
  (params (OverlappedComponent :type "PrimitiveComponent Object Reference") (OtherActor :type "Actor Object Reference") (OtherComp :type "PrimitiveComponent Object Reference") (OtherBodyIndex :type Integer) (bFromSweep :type Boolean) (SweepResult :type "HitResult Structure (by ref)"))
  (set `self.TriggeredSoul` true)
  (if (== OtherActor (`self.PlayerRef`))
    (bind (_direction _movement) (`Timeline|PickupMovement` :!via `PlayFromStart`)
      (:`Update`
        (`self.K2_SetActorLocation` (`KismetMathLibrary.VInterpTo` (`SceneComponent.K2_GetComponentLocation` (`self.healthpickup_MESH`)) (`self.K2_GetActorLocation` (`self.PlayerRef`)) _movement 0.1))))))

(event `self.ReceiveTick`
  (params (DeltaSeconds :type "Float (single-precision)"))
  (if (`self.TriggeredSoul`)
    (if (< (`KismetMathLibrary.Vector_Distance` (`SceneComponent.K2_GetComponentLocation` (`self.healthpickup_MESH`)) (`self.K2_GetActorLocation` (`self.PlayerRef`))) 600.0)
      (`HealthComponent.GainHealth` (`PlayerCharacter.HealthComponent` (`self.PlayerRef`)) 10)
      (bind _returnvalue (`FMODBlueprintStatics.PlayEvent2D` "/Game/FMOD/Events/Objects/SoulOrbPickup.SoulOrbPickup"))
      (`FMODBlueprintStatics.EventInstancePlay` _returnvalue)
      (`FMODBlueprintStatics.EventInstanceRelease` _returnvalue)
      (`self.K2_DestroyActor`)
      ;[1 1 1] FMOD Turn off Low Health filter
      (bind _asbp_grim_game_mode (cast `/Game/Blueprints/GameEssentials/BP_GrimGameMode` (`GameplayStatics.GetGameMode`)))
      (if (not (<= (`HealthComponent.CurrentHealth` (`PlayerCharacter.HealthComponent` (`self.PlayerRef`))) 20.0))
        (`/Game/Blueprints/GameEssentials/BP_GrimGameMode.TurnOffLowHealth` _asbp_grim_game_mode false)))))

(fn `UserConstructionScript`)