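; BP_TheCoinPickup is a coin pickup that adds level currency when the player character overlaps it.
; BeginPlay caches the player character and BP_GrimGameMode for the overlap check.
; On overlap it passes CurrencyAmount to the game mode, doubled if HasDoubleCoin is set.
; It then plays a 2D FMOD pickup event, releases the instance and destroys itself.
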(event `self.ReceiveActorBeginOverlap`
  (params (OtherActor :type "Actor Object Reference"))
  (bind _as_bp_grim_game_mode (`self.As BP Grim Game Mode`))
  (bind _currency_amount (`self.Currency Amount`))
  (if (== OtherActor (`self.As BP Player Character`))
    (if (`/Game/Blueprints/GameEssentials/BP_GrimGameMode.hasDoubleCoin` _as_bp_grim_game_mode)
      (`GrimGameMode.AddLevelCurrency` _as_bp_grim_game_mode (* _currency_amount 2))
      (else
        (`GrimGameMode.AddLevelCurrency` _as_bp_grim_game_mode _currency_amount)))
    (bind _returnvalue (`FMODBlueprintStatics.PlayEvent2D` "/Game/FMOD/Events/Objects/CoinPickup.CoinPickup"))
    (`FMODBlueprintStatics.EventInstancePlay` _returnvalue)
    (`FMODBlueprintStatics.EventInstanceRelease` _returnvalue)
    (`self.K2_DestroyActor`)))

(event `self.ReceiveBeginPlay`
  (bind _asbp_player_character (cast `/Game/Blueprints/Player/BP_PlayerCharacter` (`GameplayStatics.GetPlayerPawn` 0)))
  (set `self.As BP Player Character` _asbp_player_character)
  (bind _asbp_grim_game_mode (cast `/Game/Blueprints/GameEssentials/BP_GrimGameMode` (`GameplayStatics.GetGameMode`)))
  (set `self.As BP Grim Game Mode` _asbp_grim_game_mode))

(fn `UserConstructionScript`)