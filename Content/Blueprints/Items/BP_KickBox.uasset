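; BP_KickBox is a breakable, kickable urn that can drop a coin or health pickup.
; Kicking enables cube physics and breaks it after a short delay.
; Any non-player overlap flags a break on Tick, and a kicked urn also damages enemies it overlaps.
; These paths share the health death logic, which rolls loot, spawns BP_UrnBreak, plays a sound and destroys the actor.
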(event `self.Health.OnDeath`
  (bind _returnvalue (<= (`KismetMathLibrary.RandomFloatInRange` 0.0 100.0) 50.0))
  (bind _returnvalue_2 (`KismetMathLibrary.Conv_VectorToTransform` (`SceneComponent.K2_GetComponentLocation` (`self.Cube`))))
  ;[1 1 1] Push and spawn coins + particles on kick
  (`|ExecutionSequence` :!label _label
    (:`then_0`
      (if _returnvalue
        (`|SpawnActorFromClass` "/Game/Blueprints/Items/BP_TheCoinPickup.BP_TheCoinPickup_C" _returnvalue_2 "AdjustIfPossibleButAlwaysSpawn" "OverrideRootScale" null null)
        (elif _returnvalue
          (`|SpawnActorFromClass` "/Game/Blueprints/Items/BP_HealthPickup.BP_HealthPickup_C" _returnvalue_2 "AdjustIfPossibleButAlwaysSpawn" "OverrideRootScale" null null))))
    (:`then_1`
      (`|SpawnActorFromClass` "/Game/Blueprints/Environment/BP_UrnBreak.BP_UrnBreak_C" _returnvalue_2 "AdjustIfPossibleButAlwaysSpawn" "OverrideRootScale" null null)
      (`FMODBlueprintStatics.PlayEvent2D` "/Game/FMOD/Events/Objects/UrnBreak.UrnBreak")
      (`FMODBlueprintStatics.EventInstancePlay` (struct))
      (`FMODBlueprintStatics.EventInstanceRelease` (struct))
      (`self.K2_DestroyActor`))))

(event `self.ReceiveTick`
  (params (DeltaSeconds :type "Float (single-precision)"))
  ;[1 1 1] Push and spawn coins + particles on kick
  (if (`self.breakNow`)
    (goto _label)))

(event `/Game/Blueprints/Player/BI_Kick.Kick`
  ;[1 1 1] Push and spawn coins + particles on kick
  (set `self.doKick` true)
  (`PrimitiveComponent.SetSimulatePhysics` (`self.Cube`) true)
  (`KismetSystemLibrary.Delay` 0.6)
  (goto _label))

(event `self.Collider.OnComponentBeginOverlap`
  (params (OverlappedComponent :type "PrimitiveComponent Object Reference") (OtherActor :type "Actor Object Reference") (OtherComp :type "PrimitiveComponent Object Reference") (OtherBodyIndex :type Integer) (bFromSweep :type Boolean) (SweepResult :type "HitResult Structure (by ref)"))
  ;[1 1 1] Break on collision
  (`|ExecutionSequence`
    (:`then_0`
      (cast `/Game/Blueprints/Player/BP_PlayerCharacter` OtherActor ; Any collision other than player will break the pot
        (:`CastFailed`
          (set `self.breakNow` true :!label _label_2))))
    (:`then_1`
      (bind _asbp_base_enemy_new (cast `/Game/Blueprints/AI/BP_BaseEnemy_NEW` OtherActor))
      (if (`self.doKick`)
        (`HealthComponent.TakeDamage` (`BaseEnemy.HealthComponent` _asbp_base_enemy_new) 1.0 false)
        (goto _label_2)))))

(fn `UserConstructionScript`)