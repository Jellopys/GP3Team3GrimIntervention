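; Health pickup actor that heals the player character by a set amount when the player overlaps its box trigger.
; On pickup it calls GainHealth on the player's HealthComponent, destroys itself and plays a one-shot 2D FMOD soul orb sound.
; It then calls the game mode to turn off the low-health audio filter if the player's health is above the low threshold.
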(event `self.Box.OnComponentBeginOverlap`
  (params (OverlappedComponent :type "PrimitiveComponent Object Reference") (OtherActor :type "Actor Object Reference") (OtherComp :type "PrimitiveComponent Object Reference") (OtherBodyIndex :type Integer) (bFromSweep :type Boolean) (SweepResult :type "HitResult Structure (by ref)"))
  (if (== OtherActor (`self.As BP Player Character`))
    (`HealthComponent.GainHealth` (`PlayerCharacter.HealthComponent` (`self.As BP Player Character`)) (`self.Healthamount`))
    (`self.K2_DestroyActor`)
    (bind _returnvalue (`FMODBlueprintStatics.PlayEvent2D` "/Game/FMOD/Events/Objects/SoulOrbPickup.SoulOrbPickup"))
    (`FMODBlueprintStatics.EventInstancePlay` _returnvalue)
    (`FMODBlueprintStatics.EventInstanceRelease` _returnvalue)
    ;[1 1 1] FMOD Turn off Low Health filter
    (bind _asbp_grim_game_mode (cast `/Game/Blueprints/GameEssentials/BP_GrimGameMode` (`GameplayStatics.GetGameMode`)))
    (if (not (<= (`HealthComponent.CurrentHealth` (`PlayerCharacter.HealthComponent` (`self.As BP Player Character`))) 20.0))
      (`/Game/Blueprints/GameEssentials/BP_GrimGameMode.TurnOffLowHealth` _asbp_grim_game_mode false))))

(fn `UserConstructionScript`
  (`parent.UserConstructionScript`))