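; Hollow Scythe pickup, presented as trading half damage for 50% more attack speed.
; When the player character overlaps its box, it calls UpgradeStat on BP_GrimGameInstance for attack speed and the three combo damages.
; The multiply and divide inputs are literal zeros, so every upgrade value passed is zero.
; It then shows an animated power-up widget and destroys itself.
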(event `self.Box.OnComponentBeginOverlap`
  (params (OverlappedComponent :type "PrimitiveComponent Object Reference") (OtherActor :type "Actor Object Reference") (OtherComp :type "PrimitiveComponent Object Reference") (OtherBodyIndex :type Integer) (bFromSweep :type Boolean) (SweepResult :type "HitResult Structure (by ref)"))
  (if (== OtherActor (`self.As BP Player Character`))
    (bind _asbp_grim_game_instance (cast `/Game/Blueprints/GameEssentials/BP_GrimGameInstance` (`GameplayStatics.GetGameInstance`)))
    (`GrimGameInstance.UpgradeStat` _asbp_grim_game_instance (* 0.0 1.5) "AttackSpeed")
    (`GrimGameInstance.UpgradeStat` _asbp_grim_game_instance (/ 0.0 2.0) "FirstComboDamage")
    (`GrimGameInstance.UpgradeStat` _asbp_grim_game_instance (/ 0.0 2.0) "SecondComboDamage")
    (`GrimGameInstance.UpgradeStat` _asbp_grim_game_instance (/ 0.0 2.0) "ThirdComboDamage")
    ;[1 1 1] Pickup UI Info
    (bind _returnvalue (`|CreateWidget` "/Game/UI/PowerUp/UW_PowerUpDisplay.UW_PowerUpDisplay_C" (`GameplayStatics.GetPlayerController` 0)))
    (`UserWidget.AddToViewport` _returnvalue 0)
    (`PowerupCollectWidget.StartPowerUpAnimation` _returnvalue "Hollow Scythe" "Attack speed increased by 50%, Half damage" "/Game/UI/Images/office2.office2")
    (`self.K2_DestroyActor`)))

(fn `UserConstructionScript`
  (`parent.UserConstructionScript`))