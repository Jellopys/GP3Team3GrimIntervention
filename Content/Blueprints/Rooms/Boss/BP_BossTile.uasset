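; BP_BossTile is the boss room tile, handling the room's opening and the start of the boss encounter.
; OnBossRoomOpen destroys five blocker components and the Niagara door effect.
; The player's first overlap with the entry box spawns BP_Boss_NEW above the boss scenery, guarded by a one-shot flag.
; It also stops level music and atmosphere through BP_GrimGameMode, then plays boss music and a boss voice line as audio events.
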(event `self.ReceiveBeginPlay`
  (bind _asbp_player_character (cast `/Game/Blueprints/Player/BP_PlayerCharacter` (`GameplayStatics.GetPlayerPawn` 0)))
  (set `self.As BP Player Character` _asbp_player_character))

(event `self.OnBossRoomOpen`
  (`ActorComponent.K2_DestroyComponent` (`self.BossBlocker1`))
  (`ActorComponent.K2_DestroyComponent` (`self.BossBlocker2`))
  (`ActorComponent.K2_DestroyComponent` (`self.BossBlocker3`))
  (`ActorComponent.K2_DestroyComponent` (`self.BossBlocker4`))
  (`ActorComponent.K2_DestroyComponent` (`self.BossBlocker5`))
  (`ActorComponent.K2_DestroyComponent` (`self.NiagaraBossDoor`)))

(event `self.BossRoomEnterBox.OnComponentBeginOverlap`
  (params (OverlappedComponent :type "PrimitiveComponent Object Reference") (OtherActor :type "Actor Object Reference") (OtherComp :type "PrimitiveComponent Object Reference") (OtherBodyIndex :type Integer) (bFromSweep :type Boolean) (SweepResult :type "HitResult Structure (by ref)"))
  (bind (_returnvalue_x _returnvalue_y _returnvalue_z) (`KismetMathLibrary.BreakVector` (`SceneComponent.K2_GetComponentLocation` (`self.BossScenery`))))
  (if (== OtherActor (`self.As BP Player Character`))
    (if (not (`self.bossHasSpawned`))
      (`|ExecutionSequence`
        (:`then_0`
          (set `self.bossHasSpawned` true)
          (`|SpawnActorFromClass` "/Game/Blueprints/AI/BP_Boss_NEW.BP_Boss_NEW_C" (`KismetMathLibrary.Conv_VectorToTransform` (`KismetMathLibrary.MakeVector` _returnvalue_x _returnvalue_y (+ _returnvalue_z 150.0))) "Undefined" "OverrideRootScale" null null))
        (:`then_1`
          ;[1 1 1] Stop playing level music
          (bind _asbp_grim_game_mode (cast `/Game/Blueprints/GameEssentials/BP_GrimGameMode` (`GameplayStatics.GetGameMode`)))
          (`FMODBlueprintStatics.EventInstanceStop` (`/Game/Blueprints/GameEssentials/BP_GrimGameMode.LevelMusic` _asbp_grim_game_mode) true)
          ;[1 1 1] Start play boss music
          (bind _asbp_grim_game_mode_2 (cast `/Game/Blueprints/GameEssentials/BP_GrimGameMode` (`GameplayStatics.GetGameMode`)))
          (`/Game/Blueprints/GameEssentials/BP_GrimGameMode.Play Boss Music` _asbp_grim_game_mode_2)
          (bind _bossmusic (`/Game/Blueprints/GameEssentials/BP_GrimGameMode.BossMusic` _asbp_grim_game_mode_2))
          (`FMODBlueprintStatics.EventInstancePlay` _bossmusic)
          (`FMODBlueprintStatics.EventInstanceRelease` _bossmusic))
        (:`then_2`
          ;[1 1 1] Stop playing atmosphere sound
          (bind _asbp_grim_game_mode_3 (cast `/Game/Blueprints/GameEssentials/BP_GrimGameMode` (`GameplayStatics.GetGameMode`)))
          (`FMODBlueprintStatics.EventInstanceStop` (`/Game/Blueprints/GameEssentials/BP_GrimGameMode.Atmosphere` _asbp_grim_game_mode_3) true))
        (:`then_3`
          ;[1 1 1] Play boss speaks
          (bind _returnvalue (`FMODBlueprintStatics.PlayEvent2D` "/Game/FMOD/Events/Enemies/BossSpeak.BossSpeak"))
          (`FMODBlueprintStatics.EventInstancePlay` _returnvalue)
          (`FMODBlueprintStatics.EventInstanceRelease` _returnvalue))))))

(fn `UserConstructionScript`)