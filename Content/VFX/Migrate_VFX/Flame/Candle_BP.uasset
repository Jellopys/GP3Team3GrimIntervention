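; Candle flame prop Blueprint with an Enabled switch and a flicker timeline, both left unwired.
; The construction script passes Enabled to SetEnabled, whose entry leads nowhere.
; Disconnected nodes there would store the flag, toggle visibility of Serq and Serq1, and invert Candle shadow casting.
; BeginPlay is empty, so the Flickering timeline and its MinIntensity-to-MaxIntensity lerp never run.
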(event `self.ReceiveBeginPlay`)

(fn `SetEnabled`
  (params (Enabled :type Boolean)))

(fn `UserConstructionScript`
  (`self.SetEnabled` (`self.Enabled`)))