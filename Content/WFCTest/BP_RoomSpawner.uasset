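; Room spawner for a Wave Function Collapse test that starts building a tile layout on BeginPlay.
; It generates a square grid sized by GridSize with fixed tile spacing, centered below the world origin.
; It then adds every SectorClass actor in the level to SectorCounter.
; If the count exceeds one, it collapses the first tile and then calls CollapseNextTile once.
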(event `self.ReceiveBeginPlay`
  (bind _grid_size (`self.Grid Size`))
  (`self.GenerateGrid` (0.0 0.0 -1000.0) _grid_size _grid_size 1100.0)
  (bind _outactors (`GameplayStatics.GetAllActorsOfClass` (`self.SectorClass`)))
  (for _ _outactors
    (set `self.SectorCounter` (+ (`self.SectorCounter`) 1)))
  (if (> (`self.SectorCounter`) 1)
    (`self.CollapseFirstTile`)
    (`self.CollapseNextTile`)))

(fn `UserConstructionScript`)